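; BP_ProceduralMesh is an actor that builds a procedural mesh section from its Vertices and Indexes arrays, as one piece of an indexed chain.
; The construction script creates the section, then resets both arrays to a single placeholder entry.
; Pieces with an even ChainIndex get the M_WhiteSurface material, so alternate pieces can look different.
; The event graph holds only disabled stubs, so nothing runs at play time.
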(event EventBeginPlay)

(event Collision|EventActorBeginOverlap
  (params (OtherActor :type Actor%20Object%20Reference)))

(event EventTick
  (params (DeltaSeconds :type Float%20%28single-precision%29)))

(fn ConstructionScript
  (bind _proceduralmesh (Variables|Default|GetProceduralMesh))
  (Class|ProceduralMeshComponent|CreateMeshSectionLinearColor _proceduralmesh 0 (Variables|Default|GetVertices) (Variables|Default|GetIndexes) 0 0 0 0 0 0 0 false)
  (Variables|Default|SetVertices (Utilities|Array|MakeArray "0.000000, 0, 0"))
  (Variables|Default|SetIndexes (Utilities|Array|MakeArray 0))
  (if (== (Math|Integer|%(Integer) (Variables|Default|GetChain%20index) 2) 0)
    (Rendering|Material|SetMaterial _proceduralmesh 0 "/Game/Materials/M_WhiteSurface.M_WhiteSurface")))