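; BP_Residue is an actor that displays one residue, apparently part of a chain, as a procedural mesh.
; Its construction script builds a single mesh section from the Vertices and Indexes arrays, then clears both arrays.
; Residues with an even ChainIndex get the M_WhiteSurface material, while odd ones receive no material assignment here.
; The event graph holds only disabled default events, so it adds no runtime logic.
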(event EventBeginPlay)

(event Collision|EventActorBeginOverlap
  (params (OtherActor :type Actor%20Object%20Reference)))

(event EventTick
  (params (DeltaSeconds :type Float%20%28single-precision%29)))

(fn ConstructionScript
  (bind _proceduralmesh (Variables|Default|GetProceduralMesh))
  (Class|ProceduralMeshComponent|CreateMeshSectionLinearColor _proceduralmesh 0 (Variables|Default|GetVertices) (Variables|Default|GetIndexes) 0 0 0 0 0 0 0 false)
  (Utilities|Array|Clear (Variables|Default|GetVertices))
  (Utilities|Array|Clear (Variables|Default|GetIndexes))
  (if (== (Math|Integer|%(Integer) (Variables|Default|GetChain%20index) 2) 0)
    (Rendering|Material|SetMaterial _proceduralmesh 0 "/Game/Materials/M_WhiteSurface.M_WhiteSurface")))