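; BP_Atom is an actor that represents a single atom as a colored sphere in the protein viewer.
; Its construction script creates a dynamic instance of M_Atom on the sphere mesh and sets its Color parameter from the element in its Structure data, covering C, O, N, P, FE and S.
; A Set Hidden function toggles the atom's in-game visibility, and the event graph holds no active logic.
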(event EventBeginPlay)

(event Collision|EventActorBeginOverlap
  (params (OtherActor :type Actor%20Object%20Reference)))

(event EventTick
  (params (DeltaSeconds :type Float%20%28single-precision%29)))

(fn ConstructionScript
  (bind _returnvalue (Rendering|Material|CreateDynamicMaterialInstance (Variables|Default|GetSphereMesh) 0 "/Game/ProteinViewer/Biology/Atom/M_Atom.M_Atom" "None" :!class /Script/Engine.PrimitiveComponent))
  (Variables|Default|SetMaterial%20Instance _returnvalue)
  (switch string (.Element (Utilities|Struct|BreakAtomStruct (Variables|Default|GetStructure)))
    (:C
      (Variables|Default|SetColor "(R=0.291667,G=0.291667,B=0.291667,A=1.000000)"))
    (:O
      (Variables|Default|SetColor "(R=1.000000,G=0.000000,B=0.000000,A=1.000000)"))
    (:N
      (Variables|Default|SetColor "(R=0.188235,G=0.313726,B=0.972549,A=1.000000)"))
    (:P
      (Variables|Default|SetColor "(R=1.000000,G=0.501961,B=0.000000,A=1.000000)"))
    (:FE
      (Variables|Default|SetColor "(R=0.878431,G=0.400000,B=0.200000,A=1.000000)"))
    (:S
      (Variables|Default|SetColor "(R=1.000000,G=1.000000,B=0.188235,A=1.000000)")))
  (Rendering|Material|SetVectorParameterValue (Variables|Default|GetMaterial%20Instance) "Color" (Variables|Default|GetColor) :!class /Script/Engine.MaterialInstanceDynamic))

(fn SetHidden
  (params (IsHidden :type Boolean))
  (Rendering|SetActorHiddenInGame IsHidden))