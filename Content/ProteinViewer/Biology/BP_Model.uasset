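; Protein model actor that builds and controls the atom and ribbon representations of a structure.
; SpawnAtoms creates a scaled BP_Atom per atom struct, destroying earlier atoms on reload, and RenderRibbon spawns a BP_Chain per chain from its residues.
; Stored actor arrays let each representation be hidden separately and let ribbons receive random dark colors through dynamic material instances.
; Reloading never empties the Atoms array, and RenderRibbon clears Chains without destroying the old actors.
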(event EventBeginPlay)

(event Collision|EventActorBeginOverlap
  (params (OtherActor :type Actor%20Object%20Reference)))

(event EventTick
  (params (DeltaSeconds :type Float%20%28single-precision%29)))

(fn ConstructionScript)

(fn SpawnAtoms
  (params (Atom%20Structs :type Array%20of%20Atom%20Struct%20Structures))
  (if (Variables|Default|GetIs%20Model%20Loaded)
    (CallFunction|DestroyAtoms)
    (else
      (Variables|Default|SetIs%20Model%20Loaded true)))
  (for _array_element Atom%20Structs
    (bind _returnvalue (Game|SpawnActorfromClass "/Game/ProteinViewer/Biology/Atom/BP_Atom.BP_Atom_C" (Math|Conversions|ToTransform(Vector) (* (.coordinates (Utilities|Struct|BreakAtomStruct _array_element)) (Variables|Default|GetAtom%20Scale))) "AlwaysSpawn" self _array_element 0))
    (Utilities|Array|Add (Variables|Default|GetAtoms) _returnvalue)))

(fn DestroyAtoms
  (for _array_element (Variables|Default|GetAtoms)
    (Actor|DestroyActor _array_element))
  (return))

(fn RenderRibbon
  (params (Chains%20Structs :type Array%20of%20Chain%20Structures))
  (Utilities|Array|Clear (Variables|Default|GetChains))
  (for _array_element Chains%20Structs
    (bind _returnvalue (Game|SpawnActorfromClass "/Game/ProteinViewer/Biology/BP_Chain.BP_Chain_C" (Math|Transform|MakeTransform "0, 0, 0" "0, 0, 0" (Math|Conversions|ToVector(Float) (Variables|Default|GetAtom%20Scale))) "Undefined" 0 (.residues (Utilities|Struct|BreakChain _array_element)) (.chainID (Utilities|Struct|BreakChain _array_element)) 0))
    (Utilities|Array|Add (Variables|Default|GetChains) _returnvalue)))

(fn RibbonSetHidden
  (params (Is%20Hidden :type Boolean))
  (for _array_element (Variables|Default|GetChains)
    (Default|SetHidden _array_element Is%20Hidden)
    (Variables|Default|SetIsRibbonHidden Is%20Hidden)))

(fn AtomsSetHidden
  (params (Is%20Hidden :type Boolean))
  (for _array_element (Variables|Default|GetAtoms)
    (Default|SetHidden _array_element Is%20Hidden)
    (Variables|Default|SetIsAtomsHidden Is%20Hidden)))

(fn RibbonPaintRandom
  (for _array_element (Variables|Default|GetChains)
    (bind _returnvalue (Rendering|Material|CreateDynamicMaterialInstance "/Game/ProteinViewer/M_WhiteSurface.M_WhiteSurface" "None" "None" :!class /Script/Engine.KismetMaterialLibrary))
    (Rendering|Material|SetVectorParameterValue _returnvalue "Color" (Math|Color|MakeColor (Math|Random|RandomFloatinRange 0.0 0.2) (Math|Random|RandomFloatinRange 0.0 0.2) (Math|Random|RandomFloatinRange 0.0 0.2)) :!class /Script/Engine.MaterialInstanceDynamic)
    (Default|ChangeMaterialInstance _array_element _returnvalue)))