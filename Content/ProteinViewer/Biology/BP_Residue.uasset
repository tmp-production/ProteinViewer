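; Actor for a single protein residue in the protein viewer, drawn as a procedural mesh with switchable coloring.
; The construction script builds the mesh from the Vertices and Indexes arrays, then clears both.
; ColorBySecondaryStructure applies a new dynamic material tinted by Coil, Helix or Strand type, while ColorByChains applies MatRibbon, which is not assigned here.
; A TODO marks color creation for a future secondary-structure actor.
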(event EventBeginPlay)

(event Collision|EventActorBeginOverlap
  (params (OtherActor :type Actor%20Object%20Reference)))

(event EventTick
  (params (DeltaSeconds :type Float%20%28single-precision%29)))

(fn ConstructionScript
  (Class|ProceduralMeshComponent|CreateMeshSectionLinearColor (Variables|Default|GetProceduralMesh) 0 (Variables|Construction|GetVertices) (Variables|Construction|GetIndexes) 0 0 0 0 0 0 0 false)
  (Utilities|Array|Clear (Variables|Construction|GetIndexes))
  (Utilities|Array|Clear (Variables|Construction|GetVertices)))

(fn ColorbySecondaryStructure
  ;[1 0.4971 0.4193] TODO Создание цвета должно происходить в акторе для вторичной структуры, но пока его нет =(
  (bind _returnvalue (Rendering|Material|CreateDynamicMaterialInstance "/Game/ProteinViewer/M_WhiteSurface.M_WhiteSurface" "None" "None" :!class /Script/Engine.KismetMaterialLibrary))
  (Variables|Coloring|SetMat_Secondary _returnvalue)
  (switch Utilities|FlowControl|Switch|SwitchonEResidueType (Variables|Default|GetType)
    (:ResidueTypeCoil
      (Variables|Coloring|SetColor_Secondary "(R=0.000000,G=0.316667,B=0.001267,A=1.000000)"))
    (:ResidueTypeHelix
      (Variables|Coloring|SetColor_Secondary "(R=0.000000,G=0.000000,B=0.308333,A=1.000000)"))
    (:ResidueTypeStrand
      (Variables|Coloring|SetColor_Secondary "(R=0.350000,G=0.000000,B=0.000000,A=1.000000)")))
  (Rendering|Material|SetVectorParameterValue (Variables|Coloring|GetMat_Secondary) "Color" (Variables|Coloring|GetColor_Secondary) :!class /Script/Engine.MaterialInstanceDynamic)
  (Rendering|Material|SetMaterial (Variables|Default|GetProceduralMesh) 0 (Variables|Coloring|GetMat_Secondary)))

(fn ColorbyChains
  (Rendering|Material|SetMaterial (Variables|Default|GetProceduralMesh) 0 (Variables|Coloring|GetMat_Ribbon)))