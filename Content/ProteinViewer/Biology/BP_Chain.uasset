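; BP_Chain is the protein viewer's actor for one chain, built from an array of residue data.
; On BeginPlay it spawns a scaled BP_Residue at the origin per entry, passing mesh-section vertices and indices, type and index, and keeps the spawned actors.
; Functions pass a ribbon material or visibility change to every spawned residue.
; Clear empties only the residue data, leaving spawned actors in place.
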(event EventBeginPlay
  (CallFunction|SpawnResidues))

(event Collision|EventActorBeginOverlap
  (params (OtherActor :type Actor%20Object%20Reference)))

(event EventTick
  (params (DeltaSeconds :type Float%20%28single-precision%29)))

(fn ConstructionScript)

(fn SpawnResidues
  (for (_array_element _array_index) (Variables|Default|GetResidues)
    (bind _returnvalue (Game|SpawnActorfromClass "/Game/ProteinViewer/Biology/BP_Residue.BP_Residue_C" (Math|Transform|MakeTransform "0, 0, 0" "0, 0, 0" "50.000000,50.000000,50.000000") "Undefined" self (.Vertices (Utilities|Struct|BreakMeshSectionStruct (.MeshSection (Utilities|Struct|BreakResidue _array_element)))) (.Indexes (Utilities|Struct|BreakMeshSectionStruct (.MeshSection (Utilities|Struct|BreakResidue _array_element)))) _array_index (.type (Utilities|Struct|BreakResidue _array_element)) 0))
    (Utilities|Array|Add (Variables|Default|GetResidue%20Actors) _returnvalue)))

(fn ChangeMaterialInstance
  (params (Material :type Material%20Instance%20Dynamic%20Object%20Reference))
  (bind _output_get (Variables|Default|SetMaterial Material))
  (for _array_element (Variables|Default|GetResidue%20Actors)
    (Variables|/Game/ProteinViewer/Biology/BP_Residue.BP_Residue_C|SetMat_Ribbon _array_element _output_get)))

(fn Clear
  (Utilities|Array|Clear (Variables|Default|GetResidues)))

(fn Hide
  (for _array_element (Variables|Default|GetResidue%20Actors)
    (Rendering|SetActorHiddenInGame _array_element true)))

(fn Show
  (for _array_element (Variables|Default|GetResidue%20Actors)
    (Rendering|SetActorHiddenInGame _array_element false)))

(fn SetHidden
  (params (New%20Hidden :type Boolean))
  (for _array_element (Variables|Default|GetResidue%20Actors)
    (Rendering|SetActorHiddenInGame _array_element New%20Hidden)))